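; BP_HealthTest_Marble is a debug marble Blueprint for testing health changes on a possessed marble.
; On BeginPlay it binds to the main action event of PC_MasterController.
; When that input is pressed and the marble is possessed and can use its ability, FluctuateHealth toggles health through the CombatComponent, damaging by half of max health when above half, otherwise healing by the same amount.
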(event Custom|MainActionTriggered
  (params (Input :type Boolean))
  (if Input
    (CallFunction|FluctuateHealth)))

(event EventBeginPlay
  (bind _returnvalue (Actor|GetActorOfClass "/Game/NGDMP/Player/PC_MasterController.PC_MasterController_C"))
  (EventDispatchers|BindEventtoFIAMainAction _returnvalue (delegate Custom|MainActionTriggered)))

(fn ConstructionScript
  (|CallParentFunction))

(fn FluctuateHealth
  (bind _combatcomponent (Variables|Default|GetCombatComponent))
  (bind _maxhealth (Variables|/Script/NGDMP.CombatComponent|GetMaxHealth _combatcomponent))
  (bind _returnvalue (/ _maxhealth 2.0))
  (if (Variables|Default|GetbPossessed)
    (if (Variables|Default|GetCanUseAbility) ; For debug, so don't care about this
      (if (> (Variables|/Script/NGDMP.CombatComponent|GetCurrentHealth _combatcomponent) _returnvalue)
        (Class|CombatComponent|TakeDamage (Variables|Default|GetCombatComponent) _returnvalue)
        (else
          (Class|CombatComponent|Heal (Variables|Default|GetCombatComponent) _returnvalue))))))