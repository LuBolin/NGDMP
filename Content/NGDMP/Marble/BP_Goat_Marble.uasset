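; BP_Goat_Marble is a marble variant whose special ability is a forward charge.
; On BeginPlay it binds to the main action event of PC_MasterController, and that input calls Charge.
; Charge applies a velocity-change impulse to the physics mesh along the camera's forward vector, only while the marble is possessed and the ability is available, then marks the ability as used.
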(event Custom|MainActionTriggered
  (params (Input :type Boolean))
  (CallFunction|Charge))

(event EventBeginPlay
  (bind _returnvalue (Actor|GetActorOfClass "/Game/NGDMP/Player/PC_MasterController.PC_MasterController_C"))
  (EventDispatchers|BindEventtoFIAMainAction _returnvalue (delegate Custom|MainActionTriggered)))

(fn ConstructionScript
  (|CallParentFunction))

(fn Charge
  (if (Variables|Default|GetbPossessed)
    (if (Variables|Default|GetCanUseAbility)
      (Physics|AddImpulse (Variables|Default|GetPhysicsMesh) (* (Transformation|GetActorForwardVector (Game|GetPlayerCameraManager 0)) 1e+03) "None" true)
      (Variables|Default|SetCanUseAbility false))))