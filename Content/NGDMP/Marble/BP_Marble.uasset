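; BP_Marble is a marble that highlights itself when the player controller aims at or possesses it.
; On BeginPlay it finds PC_MasterController and binds to its AimUpdated and PossessUpdated events.
; Each marble compares the broadcast marble to itself, tracks a Possessed flag, and sets or clears an overlay material on its Marble component.
; Aim updates are ignored while possessed, so the possessed highlight takes priority.
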(event Custom|Aim%20Updated
  (params (AimedMarble :type Base%20Marble%20Object%20Reference))
  (bind _marble (Variables|Default|GetMarble))
  (if (not (Variables|Default|GetbPossessed))
    (if (== AimedMarble self)
      (Rendering|Material|SetOverlayMaterial _marble "/Game/NGDMP/Marble/M_MarbleAImed.M_MarbleAImed" :!class /Script/Engine.MeshComponent)
      (else
        (Rendering|Material|SetOverlayMaterial _marble 0 :!class /Script/Engine.MeshComponent)))))

(event Custom|Possess%20Updated
  (params (PossessUpdated :type Base%20Marble%20Object%20Reference))
  (bind _marble (Variables|Default|GetMarble))
  (if (== PossessUpdated self)
    (Variables|Default|SetbPossessed true)
    (Rendering|Material|SetOverlayMaterial _marble "/Game/NGDMP/Marble/M_MarblePossessed.M_MarblePossessed" :!class /Script/Engine.MeshComponent)
    (else
      (Variables|Default|SetbPossessed false)
      (Rendering|Material|SetOverlayMaterial _marble 0 :!class /Script/Engine.MeshComponent))))

(event EventBeginPlay
  (bind _returnvalue (Actor|GetActorOfClass "/Game/NGDMP/Player/PC_MasterController.PC_MasterController_C"))
  (Variables|Default|SetParentController _returnvalue)
  (EventDispatchers|BindEventtoAimUpdated (Variables|Default|GetParentController) (delegate Custom|Aim%20Updated))
  (EventDispatchers|BindEventtoPossessUpdated (Variables|Default|GetParentController) (delegate Custom|Possess%20Updated)))

(fn ConstructionScript)