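; BP_Cow_Marble is a cow marble variant whose special ability is a jump.
; On BeginPlay it binds to the use-ability delegate, which calls Jump.
; Jump requires the marble to be possessed and the ability available, then applies an upward velocity-change impulse scaled by JumpForce to the physics mesh.
; It then clears CanUseAbility, and nothing in this graph restores it.
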(event Custom|AbilityTriggered
  (CallFunction|Jump))

(event EventBeginPlay
  (EventDispatchers|BindEventtoFonUseAbility (delegate Custom|AbilityTriggered)))

(fn ConstructionScript
  (|CallParentFunction))

(fn Jump
  (if (Variables|Default|GetbPossessed)
    (if (Variables|Default|GetbCanUseAbility)
      (Physics|AddImpulse (Variables|Default|GetPhysicsMesh) (* (Math|Vector|VectorUp) (Variables|Default|GetJumpForce)) "None" true)
      (Variables|Default|SetbCanUseAbility false))))