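; BP_Goat_Marble is a goat-themed marble Blueprint whose ability is a forward charge.
; On BeginPlay it binds the parent's use-ability event to Charge.
; Charge runs only when the marble is possessed and the ability is available, applying a mass-independent impulse to the physics mesh along the player camera's forward vector.
; It then clears the availability flag, which this Blueprint never resets itself.
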(event Custom|AbilityTriggered
  (CallFunction|Charge))

(event EventBeginPlay
  (EventDispatchers|BindEventtoFonUseAbility (delegate Custom|AbilityTriggered)))

(fn ConstructionScript
  (|CallParentFunction))

(fn Charge
  (if (Variables|Default|GetbPossessed)
    (if (Variables|Default|GetbCanUseAbility)
      (Physics|AddImpulse (Variables|Default|GetPhysicsMesh) (* (Transformation|GetActorForwardVector (Game|GetPlayerCameraManager 0)) 1e+03) "None" true)
      (Variables|Default|SetbCanUseAbility false))))