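; BP_Crab_Marble is a crab animal marble whose ability is a brake.
; It binds to the start-acting and use-ability events, then attempts a brake on BeginPlay.
; Braking requires possession and an available ability, then applies brake linear damping to the physics mesh and consumes the ability.
; Launching restores default damping but does not re-arm the ability in this Blueprint.
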(event Custom|AbilityTriggered
  (CallFunction|Brake))

(event Custom|Launched
  (CallFunction|ResetBrake))

(event EventBeginPlay
  (EventDispatchers|BindEventtoFonStartActing (delegate Custom|Launched))
  (EventDispatchers|BindEventtoFonUseAbility (delegate Custom|AbilityTriggered))
  (CallFunction|Brake))

(fn ConstructionScript
  (|CallParentFunction))

(fn Brake
  (if (Variables|Default|GetbPossessed)
    (if (Variables|Default|GetbCanUseAbility)
      (Class|PrimitiveComponent|SetLinearDamping (Variables|Default|GetPhysicsMesh) (Variables|Default|GetBrakeDamping))
      (Variables|Default|SetbCanUseAbility false))))

(fn ResetBrake
  (Class|PrimitiveComponent|SetLinearDamping (Variables|Default|GetPhysicsMesh) (Variables|Default|GetDefaultDamping)))