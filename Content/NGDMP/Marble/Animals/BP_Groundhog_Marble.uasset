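; Groundhog marble Blueprint whose ability is a roar, fired along the camera's forward direction.
; When the use-ability event fires on a possessed marble with the ability available, ConeBasedRoar clears availability and spawns BP_Groundhog_Roar.
; The spawn point is offset forward so the cone naturally pushes the groundhog backwards.
; An unused Roar function holds a trace-based alternative with cone-filtered impulses and self-recoil.
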(event Custom|AbilityTriggered
  (CallFunction|ConeBasedRoar))

(event EventBeginPlay
  (EventDispatchers|BindEventtoFonUseAbility (delegate Custom|AbilityTriggered)))

(fn ConstructionScript
  (|CallParentFunction))

(fn Roar
  (bind _returnvalue (Transformation|GetActorLocation))
  (bind _returnvalue_2 (Transformation|GetActorLocation))
  (if (Variables|Default|GetbPossessed)
    (if (Variables|Default|GetbCanUseAbility)
      (LocalVariables|SetForward (Transformation|GetActorForwardVector (Game|GetPlayerCameraManager 0)))
      (Variables|Default|SetbCanUseAbility false)
      (bind _outhits (Collision|MultiSphereTraceForObjects _returnvalue (+ _returnvalue (* (LocalVariables|GetForward) (LocalVariables|GetRoarRange))) (LocalVariables|GetRoarRange) (Utilities|Array|MakeArray "ObjectTypeQuery4") false 0 "None"))
      (for _array_element _outhits
        ;[0.15 0.15 0.15 0.5] Launch Entities
        (bind _angle (CallFunction|AngleBetween2Vectors (LocalVariables|GetForward) (- (.ImpactPoint (Collision|BreakHitResult _array_element)) (Transformation|GetActorLocation))))
        (if (<= _angle (LocalVariables|GetConeAngleDegree))
          (Physics|AddImpulse (.HitComponent (Collision|BreakHitResult _array_element)) (* (Math|Vector|Normalize (- (.ImpactPoint (Collision|BreakHitResult _array_element)) (Transformation|GetActorLocation))) (* (/ (Math|Vector|VectorLength (- (.ImpactPoint (Collision|BreakHitResult _array_element)) (Transformation|GetActorLocation))) (LocalVariables|GetRoarRange)) (LocalVariables|GetMaxPushForce))) "None" true)))
      ;[0.15 0.15 0.15 0.5] Launch Self
      (bind (_outhit _returnvalue_3) (Collision|LineTraceForObjects _returnvalue_2 (+ _returnvalue_2 (* (LocalVariables|GetForward) "")) (Utilities|Array|MakeArray "ObjectTypeQuery1") false 0 "None"))
      (if _returnvalue_3
        (Physics|AddImpulse (Variables|Default|GetPhysicsMesh) (* (* (LocalVariables|GetForward) (+ (* (/ (.Distance (Collision|BreakHitResult _outhit)) 0.0) (LocalVariables|GetMaxPushForce)) (LocalVariables|GetDefaultPushBackForce))) -1.0) "None" true)))))

(fn AngleBetween2Vectors
  (params (Vec1 :type Vector) (Vec2 :type Vector))
  (return (Class|KismetMathLibrary|DegAcos (Math|Vector|DotProduct (Math|Vector|Normalize Vec1) (Math|Vector|Normalize Vec2)))))

(fn ConeBasedRoar
  (bind _returnvalue (Transformation|GetActorLocation))
  (if (Variables|Default|GetbPossessed)
    (if (Variables|Default|GetbCanUseAbility)
      (LocalVariables|SetForward (Transformation|GetActorForwardVector (Game|GetPlayerCameraManager 0)))
      (Variables|Default|SetbCanUseAbility false)
      (Game|SpawnActorfromClass "/Game/NGDMP/Marble/Animals/BP_Groundhog_Roar.BP_Groundhog_Roar_C" (Math|Transform|MakeTransform (+ _returnvalue (LocalVariables|GetForward)) (Math|Rotator|FindRelativeLookatRotation (Math|Conversions|ToTransform(Vector) _returnvalue) (+ _returnvalue (LocalVariables|GetForward)))) "Undefined" "MultiplyWithRoot" 0 0))))