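; BP_Groundhog_Roar is a short-lived groundhog roar cone that knocks objects away as it expands.
; A timeline scales it up, and overlaps during that phase give simulating objects a velocity-change impulse away from ConeForceOrigin with upward lift.
; Non-simulating crab marbles first get physics enabled and a brief no-brake window.
; After a hold, it moves its pivot to the far end, shrinks along Z and destroys itself.
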(event OnComponentBeginOverlap(Cone)
  (params (OverlappedComponent :type Primitive%20Component%20Object%20Reference) (OtherActor :type Actor%20Object%20Reference) (OtherComp :type Primitive%20Component%20Object%20Reference) (OtherBodyIndex :type Integer) (bFromSweep :type Boolean) (SweepResult :type Hit%20Result%20Structure%20%28by%20ref%29))
  (bind _rootcomponent (Variables|/Script/Engine.Actor|GetRootComponent OtherActor))
  (if (Variables|Default|GetExpanding)
    (if (Physics|IsSimulatingPhysics _rootcomponent "None")
      (if (not (Utilities|Set|Contains (Variables|Default|GetPushedObjects) OtherActor))
        (Utilities|Set|Add (Variables|Default|GetPushedObjects) _rootcomponent)
        (Physics|AddImpulse OtherComp (+ (* (Math|Vector|Normalize (- (Transformation|GetWorldLocation _rootcomponent) (Transformation|GetWorldLocation (Variables|Default|GetConeForceOrigin)))) (Variables|Default|GetPushForce)) (Variables|Default|GetBaseUpwardsForce)) "None" true :!label _label))
      (else
        (bind _asbp_crab_marble (Utilities|Casting|CastToBP_Crab_Marble OtherActor))
        (Physics|SetSimulatePhysics (Variables|/Script/NGDMP.BaseMarble|GetPhysicsMesh _asbp_crab_marble) true)
        (Variables|/Game/NGDMP/Marble/Animals/BP_Crab_Marble.BP_Crab_Marble_C|SetForceNoBrakeDurn _asbp_crab_marble 0.2)
        (goto _label)))))

(event EventBeginPlay
  (bind _coneroot (Variables|Default|GetConeRoot))
  (bind _cone (Variables|Default|GetCone))
  (bind _returnvalue (Transformation|GetWorldLocation _coneroot))
  (Transformation|SetWorldScale3D (Variables|Default|GetConeRoot) "0.010000,0.010000,0.010000")
  (Variables|Default|SetExpanding true)
  (bind _scaleuptimeline (Timeline|ScaleUp PlayFromStart)
    (:Update
      (Transformation|SetWorldScale3D (Variables|Default|GetConeRoot) (Math|Conversions|ToVector(Float) _scaleuptimeline)))
    (:Finished
      (Variables|Default|SetExpanding false)
      (Utilities|FlowControl|Delay (Variables|Default|GetMaxSizeDurn))
      (Transformation|SetWorldLocation _coneroot (+ _returnvalue (* (- (Transformation|GetWorldLocation (Variables|Default|GetCone)) _returnvalue) 2.0)) false true)
      (Transformation|SetRelativeLocation _cone (* (Variables|/Script/Engine.SceneComponent|GetRelativeLocation _cone) -1.0) false true)
      (bind _scaleuptimeline_2 (Timeline|ScaleDownTimeline ReverseFromEnd)
        (:Update
          (Transformation|SetWorldScale3D (Variables|Default|GetConeRoot) (Math|Vector|MakeVector 1.0 1.0 _scaleuptimeline_2)))
        (:Finished
          (Actor|DestroyActor))))))

(fn ConstructionScript)