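; BP_Cow_Marble is a marble Blueprint whose ability is a jump.
; On BeginPlay it finds the PC_MasterController actor and binds to its main action event, which calls Jump.
; Jump applies an upward velocity-change impulse to the physics mesh only while the marble is possessed and the ability is available, then clears the ability flag.
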(event Custom|MainActionTriggered
  (params (Input :type Boolean))
  (CallFunction|Jump))

(event EventBeginPlay
  (bind _returnvalue (Actor|GetActorOfClass "/Game/NGDMP/Player/PC_MasterController.PC_MasterController_C"))
  (EventDispatchers|BindEventtoFIAMainAction _returnvalue (delegate Custom|MainActionTriggered)))

(fn ConstructionScript
  (|CallParentFunction))

(fn Jump
  (if (Variables|Default|GetbPossessed)
    (if (Variables|Default|GetCanUseAbility)
      (Physics|AddImpulse (Variables|Default|GetPhysicsMesh) (* (Math|Vector|VectorUp) 1e+03) "None" true)
      (Variables|Default|SetCanUseAbility false))))