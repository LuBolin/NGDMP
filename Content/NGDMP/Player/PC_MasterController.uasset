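; PC_MasterController is the player controller that sets up input and the crosshair HUD for the player.
; On BeginPlay it adds the master Enhanced Input mapping context and puts a crosshair widget on the viewport.
; It forwards move, look, toggle, escape, interact and main-action input to matching CallFIA functions, with main action firing on both press and release.
; It also supplies a fixed maximum raycast distance.
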(event Input|EnhancedActionEvents|EnhancedInputActionIA_Interact
  (params (ActionValue :type Boolean) (ElapsedSeconds :type Float%20%28double-precision%29) (TriggeredSeconds :type Float%20%28double-precision%29) (InputAction :type Input%20Action%20Object%20Reference :default "/Game/NGDMP/Player/Actions/IA_Interact.IA_Interact"))
  ;[1 1 1] Input Events
  (:Started
    (Default|CallFIAInteract ActionValue)))

(event Input|EnhancedActionEvents|EnhancedInputActionIA_MasterLook
  (params (ActionValue :type Vector%202D%20Structure) (ElapsedSeconds :type Float%20%28double-precision%29) (TriggeredSeconds :type Float%20%28double-precision%29) (InputAction :type Input%20Action%20Object%20Reference :default "/Game/NGDMP/Player/Actions/IA_MasterLook.IA_MasterLook"))
  ;[1 1 1] Input Events
  (Default|CallFIAMouseLook ActionValue))

(event Input|EnhancedActionEvents|EnhancedInputActionIA_MasterMovement
  (params (ActionValue :type Vector :default "0, 0, 0") (ElapsedSeconds :type Float%20%28double-precision%29) (TriggeredSeconds :type Float%20%28double-precision%29) (InputAction :type Input%20Action%20Object%20Reference :default "/Game/NGDMP/Player/Actions/IA_MasterMovement.IA_MasterMovement"))
  ;[1 1 1] Input Events
  (Default|CallFIAMove ActionValue))

(event Input|EnhancedActionEvents|EnhancedInputActionIA_Escape
  (params (ActionValue :type Boolean) (ElapsedSeconds :type Float%20%28double-precision%29) (TriggeredSeconds :type Float%20%28double-precision%29) (InputAction :type Input%20Action%20Object%20Reference :default "/Game/NGDMP/Player/Actions/IA_Escape.IA_Escape"))
  ;[1 1 1] Input Events
  (:Started
    (Default|CallFIAEscape ActionValue)))

(event Input|EnhancedActionEvents|EnhancedInputActionIA_Toggle
  (params (ActionValue :type Boolean) (ElapsedSeconds :type Float%20%28double-precision%29) (TriggeredSeconds :type Float%20%28double-precision%29) (InputAction :type Input%20Action%20Object%20Reference :default "/Game/NGDMP/Player/Actions/IA_Toggle.IA_Toggle"))
  ;[1 1 1] Input Events
  (:Started
    (Default|CallFIAToggle ActionValue)))

(event Input|EnhancedActionEvents|EnhancedInputActionIA_MainAction
  (params (ActionValue :type Boolean) (ElapsedSeconds :type Float%20%28double-precision%29) (TriggeredSeconds :type Float%20%28double-precision%29) (InputAction :type Input%20Action%20Object%20Reference :default "/Game/NGDMP/Player/Actions/IA_MainAction.IA_MainAction"))
  ;[1 1 1] Input Events
  (:Started
    (Default|CallFIAMainAction ActionValue :!label _label))
  (:Completed
    (goto _label)))

(event EventBeginPlay
  ;[1 1 1] Init
  (Input|AddMappingContext (PlayerController|LocalPlayerSubsystems|GetEnhancedInputLocalPlayerSubsystem self) "/Game/NGDMP/Player/IMC_MasterInput.IMC_MasterInput" 0 "(bIgnoreAllPressedKeysUntilRelease=True,bForceImmediately=False,bNotifyUserSettings=False)")
  (bind _returnvalue (UserInterface|CreateWidget "/Game/NGDMP/UI/WB_Crosshair.WB_Crosshair_C"))
  (UserInterface|Viewport|AddtoViewport _returnvalue 0))

(fn ConstructionScript)

(fn GetRaycastMaxDist
  (return 1e+03))